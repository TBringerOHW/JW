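; BP_BaseEnemy is a base enemy with a health bar widget that explodes on death and then revives in place.
; BeginPlay initializes the bar and binds damage and death events, with damage refreshing the bar.
; Death spawns an explosion, hides the actor after a delay, then restores visibility and health as a timeline animates the cylinder's height.
; Tick turns the widget toward the player character.
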(event Custom|HandleDeath
  (params (Entity :type Actor%20Object%20Reference))
  (Effects|SpawnEmitteratLocation "/Game/StarterContent/Particles/P_Explosion.P_Explosion" (Transformation|GetActorLocation) "0, 0, 0" "3.000000,3.000000,3.000000")
  (Utilities|FlowControl|Delay 1.0)
  (Rendering|SetActorHiddenInGame true)
  (Utilities|FlowControl|Delay 3.0)
  (Rendering|SetActorHiddenInGame false)
  (Variables|Default|SetHealth (Variables|Default|GetMaxHealth))
  (Default|Update (Variables|Default|GetHealthBar) (Variables|Default|GetHealth) (Variables|Default|GetMaxHealth))
  (bind _value (Timeline|Revive PlayFromStart)
    (:Update
      (Transformation|SetRelativeLocation (Variables|Default|GetCylinder) (Math|Vector|MakeVector 0.0 0.0 _value) false false))))

(event EventBeginPlay
  (Utilities|FlowControl|Sequence
    (:then_0
      (bind _aswbp_health_bar (Utilities|Casting|CastToWBP_HealthBar (UserInterface|GetUserWidgetObject (Variables|Default|GetWidget))))
      (bind _output_get (Variables|Default|SetHealthBar _aswbp_health_bar))
      (Default|Init _output_get "Enemy")
      (Default|Update (Variables|Default|GetHealthBar) (Variables|Default|GetHealth) (Variables|Default|GetMaxHealth)))
    (:then_1
      (EventDispatchers|BindEventtoOnDamageReceived (EventDispatchers|CreateEvent :!event HandleDamageReceived))
      (EventDispatchers|BindEventtoOnEntityDead (EventDispatchers|CreateEvent :!event Custom|HandleDeath)))))

(event Collision|EventActorBeginOverlap
  (params (OtherActor :type Actor%20Object%20Reference)))

(event EventTick
  (params (DeltaSeconds :type Float%20%28single-precision%29))
  (Transformation|SetWorldRotation (Variables|Default|GetWidget) (Math|Rotator|FindLookatRotation (Transformation|GetActorLocation) (Transformation|GetActorLocation (Game|GetPlayerCharacter 0))) false false))

(fn ConstructionScript)

(fn HandleDamageReceived
  (params (CurrentHealth :type Float%20%28single-precision%29) (DamageAmount :type Float%20%28single-precision%29))
  (Default|Update (Variables|Default|GetHealthBar) (Variables|Default|GetHealth) (Variables|Default|GetMaxHealth)))