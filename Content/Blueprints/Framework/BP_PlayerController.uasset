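; Player controller Blueprint that sets up combat statistics tracking for the first-person character.
; On BeginPlay it hands the character HUD's stats widget to its BPStatisticsCollectorComponent.
; It then gathers every actor implementing the Damageable interface and initializes the collector with them.
; Possess only calls the parent, and Tick is unused.
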(event EventBeginPlay
  (|CallParentFunction)
  (Utilities|FlowControl|Sequence
    (:then_0
      (bind _asbp_first_person_character (Utilities|Casting|CastToBP_FirstPersonCharacter (Game|GetPlayerCharacter 0)))
      (Variables|/Game/Blueprints/BP_StatisticsCollectorComponent.BP_StatisticsCollectorComponent_C|SetWBP_Stats (Variables|Default|GetBP_StatisticsCollectorComponent) (Variables|/Game/Blueprints/Widgets/WBP_HUD.WBP_HUD_C|GetWBP_Stats (Variables|/Game/Blueprints/BP_FirstPersonCharacter.BP_FirstPersonCharacter_C|GetHUD _asbp_first_person_character))))
    (:then_1
      (bind _outactors (Actor|GetAllActorswithInterface "/Script/JW.Damageable"))
      (Class|StatisticsCollectorComponent|Initialize (Variables|Default|GetBP_StatisticsCollectorComponent) _outactors))))

(event EventTick
  (params (DeltaSeconds :type Float%20%28single-precision%29)))

(event EventPossess
  (params (PossessedPawn :type Pawn%20Object%20Reference))
  (|CallParentFunction PossessedPawn))

(fn ConstructionScript)