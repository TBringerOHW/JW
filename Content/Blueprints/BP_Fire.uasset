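; BP_Fire is a fire hazard that damages actors implementing the Damageable interface while they are inside its capsule.
; Capsule overlap begin and end events maintain the ActorsInFire list, and HandleFireDamage sends FireDamage to each entry through ReceiveDamageMessage.
; BeginPlay starts a very fast looping timer through a created event, whose bound function is not shown, instead of using Tick.
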(event OnComponentBeginOverlap(Capsule)
  (params (OverlappedComponent :type Primitive%20Component%20Object%20Reference) (OtherActor :type Actor%20Object%20Reference) (OtherComp :type Primitive%20Component%20Object%20Reference) (OtherBodyIndex :type Integer) (bFromSweep :type Boolean) (SweepResult :type Hit%20Result%20Structure%20%28by%20ref%29))
  (if (Utilities|DoesObjectImplementInterface OtherActor "/Script/JW.Damageable")
    (Utilities|Array|Add (Variables|Default|GetActorsInFire) OtherActor)))

(event OnComponentEndOverlap(Capsule)
  (params (OverlappedComponent :type Primitive%20Component%20Object%20Reference) (OtherActor :type Actor%20Object%20Reference) (OtherComp :type Primitive%20Component%20Object%20Reference) (OtherBodyIndex :type Integer))
  (if (Utilities|DoesObjectImplementInterface OtherActor "/Script/JW.Damageable")
    (Utilities|Array|RemoveItem (Variables|Default|GetActorsInFire) OtherActor)))

(event EventBeginPlay
  (Utilities|Time|SetTimerbyEvent (EventDispatchers|CreateEvent :!event HandleFireDamage) 0.01 true))

(event Collision|EventActorBeginOverlap
  (params (OtherActor :type Actor%20Object%20Reference)))

(event EventTick
  (params (DeltaSeconds :type Float%20%28single-precision%29)))

(fn ConstructionScript)

(fn HandleFireDamage
  (for _array_element (Variables|Default|GetActorsInFire)
    (Class|Damageable|ReceiveDamage(Message) _array_element (Variables|Default|GetFireDamage))))