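; BP_StatisticsCollectorComponent is an actor component that tracks combat statistics for the game: total damage dealt and enemies killed.
; HandleDamageDealt adds each damage amount to a running total and pushes it to the WBPStats widget through UpdateDamage.
; HandleEntityDeath increments the kill count and sends it to the same widget as the score.
; The event graph is empty, so both handlers rely on being invoked from outside this graph.
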(event EventBeginPlay)

(event EventTick
  (params (DeltaSeconds :type Float%20%28single-precision%29)))

(fn HandleDamageDealt
  (params (CurrentHealth :type Float%20%28single-precision%29) (DamageAmount :type Float%20%28single-precision%29))
  (bind _output_get (Variables|Default|SetTotalDealtDamage (+ (Variables|Default|GetTotalDealtDamage) DamageAmount)))
  (Default|UpdateDamage (Variables|Default|GetWBP_Stats) _output_get))

(fn HandleEntityDeath
  (params (DeadActor :type Actor%20Object%20Reference))
  (bind _result (Math|Integer|IncrementInt (Variables|Default|GetKilledEnemies))
    (:%20%20
      (Default|UpdateScore (Variables|Default|GetWBP_Stats) (Math|Conversions|ToFloat(Integer) _result)))))